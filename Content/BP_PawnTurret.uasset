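; BP_PawnTurret is an enemy turret that shoots at the player's BP_PawnTank and can be destroyed.
; While IsPatrolling is set, Tick rotates the turret mesh toward the tank.
; A looping timer line-traces from the muzzle to the tank, spawning a BP_Bullet when it hits a Player-tagged actor, with no explicit distance check.
; Damage reduces Health, and at zero it spawns a death effect and destroys itself.
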(event Custom|OnTakeAnyDamage_Event
  (params (DamagedActor :type Actor%20Object%20Reference) (Damage :type Float%20%28single-precision%29) (DamageType :type Damage%20Type%20Object%20Reference) (InstigatedBy :type Controller%20Object%20Reference) (DamageCauser :type Actor%20Object%20Reference))
  (bind _output_get (Variables|Default|SetHealth (- (Variables|Default|GetHealth) Damage)))
  (if (<= _output_get 0.0)
    (Effects|SpawnEmitteratLocation "/Game/Assets/Effects/P_DeathEffect.P_DeathEffect" (Transformation|GetActorLocation))
    (Actor|DestroyActor)))

(event EventBeginPlay
  (|CallParentFunction)
  (bind _returnvalue (Actor|GetActorOfClass "/Game/BP_PawnTank.BP_PawnTank_C"))
  (Variables|Default|SetPawnTankRef _returnvalue)
  (EventDispatchers|BindEventtoOnTakeAnyDamage (delegate Custom|OnTakeAnyDamage_Event))
  (Utilities|Time|SetTimerbyFunctionName 0 "CheckPlayerOnRange" 3.0 true))

(event Collision|EventActorBeginOverlap
  (params (OtherActor :type Actor%20Object%20Reference))
  (|CallParentFunction OtherActor) ; This node is disabled and will not be called.\nDrag off pins to build functionality.
)

(event EventTick
  (params (DeltaSeconds :type Float%20%28single-precision%29))
  (|CallParentFunction DeltaSeconds)
  (bind _pawntankref (Variables|Default|GetPawnTankRef)
    (:then
      (if (Variables|Default|GetIsPatrolling)
        (Transformation|SetWorldRotation (Variables|Default|GetTurretMesh) (Math|Rotator|FindLookatRotation (Transformation|GetActorLocation) (Transformation|GetActorLocation _pawntankref)) false false)))
    (:else)))

(fn ConstructionScript
  (|CallParentFunction))

(fn CheckPlayeronRange
  (bind _pawntankref (Variables|Default|GetPawnTankRef)
    (:then
      (bind (_outhit _returnvalue) (Collision|LineTraceByChannel (Transformation|GetWorldLocation (Variables|Default|GetProjectileSpawnPoint)) (Transformation|GetActorLocation _pawntankref) "TraceTypeQuery1" false 0 "ForDuration"))
      (if (and _returnvalue (Actor|ActorHasTag (.HitActor (Collision|BreakHitResult _outhit)) "Player"))
        (Development|PrintString "In range")
        (Game|SpawnActorfromClass "/Game/BP_Bullet.BP_Bullet_C" (Transformation|GetWorldTransform (Variables|Default|GetProjectileSpawnPoint)) "Undefined" "MultiplyWithRoot" 0 "Player" 0)))
    (:else)))