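; Player-controlled tank pawn that drives, rotates its turret and fires bullets tagged to target enemies.
; Enhanced Input events store direction values and flags that Tick turns into swept movement, body yaw and turret yaw, with steering inverted while reversing.
; Fire spawns BP_Bullet at the projectile spawn point.
; Any damage lowers Health and updates the HUD widget created at BeginPlay, with a particle effect and destruction at zero.
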(event Custom|OnTakeAnyDamage_Event
  (params (DamagedActor :type Actor%20Object%20Reference) (Damage :type Float%20%28single-precision%29) (DamageType :type Damage%20Type%20Object%20Reference) (InstigatedBy :type Controller%20Object%20Reference) (DamageCauser :type Actor%20Object%20Reference))
  (bind _output_get (Variables|Default|SetHealth (- (Variables|Default|GetHealth) Damage)))
  (Rendering|Components|TextRender|SetText (Variables|/Game/UW_Health.UW_Health_C|GetTextBlock_0 (Variables|Default|GetHealthWidget)) (Utilities|Text|ToText(String) (Utilities|String|BuildString(Integer) "Salud: " "" (Math|Float|Truncate _output_get))))
  (if (<= _output_get 0.0)
    (Effects|SpawnEmitteratLocation "/Game/Assets/Effects/P_DeathEffect.P_DeathEffect" (Transformation|GetActorLocation))
    (Actor|DestroyActor)))

(event Input|EnhancedActionEvents|EnhancedInputActionIA_MoveForward
  (params (ActionValue :type Float%20%28double-precision%29) (ElapsedSeconds :type Float%20%28double-precision%29) (TriggeredSeconds :type Float%20%28double-precision%29) (InputAction :type Input%20Action%20Object%20Reference :default "/Game/IA_MoveForward.IA_MoveForward"))
  (:Started
    (Variables|Default|SetDirection ActionValue)
    (Variables|Default|SetIsMoving true))
  (:Completed
    (Variables|Default|SetIsMoving false)))

(event Input|EnhancedActionEvents|EnhancedInputActionIA_Turn
  (params (ActionValue :type Float%20%28double-precision%29) (ElapsedSeconds :type Float%20%28double-precision%29) (TriggeredSeconds :type Float%20%28double-precision%29) (InputAction :type Input%20Action%20Object%20Reference :default "/Game/IA_Turn.IA_Turn"))
  (:Started
    (Variables|Default|SetTurnDirection ActionValue)
    (Variables|Default|SetIsTurning true))
  (:Completed
    (Variables|Default|SetIsTurning false)))

(event Input|EnhancedActionEvents|EnhancedInputActionIA_RotateTurret
  (params (ActionValue :type Float%20%28double-precision%29) (ElapsedSeconds :type Float%20%28double-precision%29) (TriggeredSeconds :type Float%20%28double-precision%29) (InputAction :type Input%20Action%20Object%20Reference :default "/Game/IA_RotateTurret.IA_RotateTurret"))
  (:Started
    (Variables|Default|SetTurretRotationDirection ActionValue)
    (Variables|Default|SetIsRotatingTurret true))
  (:Completed
    (Variables|Default|SetIsRotatingTurret false)))

(event Input|EnhancedActionEvents|EnhancedInputActionIA_Fire
  (params (ActionValue :type Boolean) (ElapsedSeconds :type Float%20%28double-precision%29) (TriggeredSeconds :type Float%20%28double-precision%29) (InputAction :type Input%20Action%20Object%20Reference :default "/Game/IA_Fire.IA_Fire"))
  (:Started
    (Game|SpawnActorfromClass "/Game/BP_Bullet.BP_Bullet_C" (Transformation|GetWorldTransform (Variables|Default|GetProjectileSpawnPoint)) "Undefined" "MultiplyWithRoot" 0 "Enemy" 0)))

(event EventBeginPlay
  (|CallParentFunction)
  (bind _asplayer_controller (Utilities|Casting|CastToPlayerController (Pawn|GetController)))
  (Utilities|IsValid (PlayerController|LocalPlayerSubsystems|GetEnhancedInputLocalPlayerSubsystem _asplayer_controller)
    (:Is%20Valid
      (Input|AddMappingContext (PlayerController|LocalPlayerSubsystems|GetEnhancedInputLocalPlayerSubsystem _asplayer_controller) "/Game/IM_Game.IM_Game" 0 "(bIgnoreAllPressedKeysUntilRelease=True,bForceImmediately=False,bNotifyUserSettings=False)")
      (EventDispatchers|BindEventtoOnTakeAnyDamage (delegate Custom|OnTakeAnyDamage_Event))
      (bind _returnvalue (UserInterface|CreateWidget "/Game/UW_Health.UW_Health_C" (Pawn|GetLocalViewingPlayerController)))
      (bind _output_get (Variables|Default|SetHealthWidget _returnvalue))
      (UserInterface|Viewport|AddtoViewport _output_get 0))))

(event Collision|EventActorBeginOverlap
  (params (OtherActor :type Actor%20Object%20Reference))
  (|CallParentFunction OtherActor) ; This node is disabled and will not be called.\nDrag off pins to build functionality.
)

(event EventTick
  (params (DeltaSeconds :type Float%20%28single-precision%29))
  (|CallParentFunction DeltaSeconds)
  (CallFunction|MoveForward DeltaSeconds)
  (CallFunction|Turn DeltaSeconds)
  (if (Variables|Default|GetIsRotatingTurret)
    (Transformation|AddLocalRotation (Variables|Default|GetTurretMesh) (Math|Rotator|MakeRotator 0.0 0.0 (* DeltaSeconds 1.5e+02 (Variables|Default|GetTurretRotationDirection))) false false)))

(fn ConstructionScript
  (|CallParentFunction))

(fn MoveForward
  (params (DeltaSeconds :type Float%20%28single-precision%29))
  (if (Variables|Default|GetIsMoving)
    (Transformation|AddActorLocalOffset (* (Math|Vector|MakeVector (Variables|Default|GetDirection) 0.0 0.0) 3e+02 DeltaSeconds) true false)))

(fn Turn
  (params (DeltaSeconds :type Float%20%28double-precision%29))
  (bind _turndirection (Variables|Default|GetTurnDirection))
  (if (Variables|Default|GetIsTurning)
    (Transformation|AddActorLocalRotation (Math|Rotator|MakeRotator 0.0 0.0 (* DeltaSeconds 2e+02 (Math|Float|SelectFloat (* _turndirection -1.0) _turndirection (and (Variables|Default|GetIsMoving) (== (Variables|Default|GetDirection) -1.0))))) false false)))